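; BP_UserController handles mouse picking on SculptedObject actors, querying which vertices fall under a brush.
; On left click it line-traces from MainCamera along the deprojected cursor direction on the Visibility channel.
; A hit on a SculptedObject draws a debug sphere at the impact point and passes that point and a fixed brush radius to VerticiesInRange.
; The result is only printed; no vertices are modified here.
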(event `Key|LeftMouseButton`
  (params (Key :type "Key Structure"))
  (bind _returnvalue (`SceneComponent.K2_GetComponentLocation` (`self.MainCamera`)))
  (:`Pressed`
    (bind (_outhit _returnvalue_2) (`KismetSystemLibrary.LineTraceSingle` _returnvalue (+ _returnvalue (* (`.WorldDirection` (`PlayerController.DeprojectMousePositionToWorld` (`GameplayStatics.GetPlayerController` 0))) 1000.0)) "TraceTypeQuery1"))
    (if _returnvalue_2
      (bind (_bblockinghit _binitialoverlap _time _distance _location _impactpoint _normal _impactnormal _physmat _hitactor _hitcomponent _hitbonename _hititem _faceindex) (`GameplayStatics.BreakHitResult` _outhit))
      (bind _assculpted_object (cast `SculptedObject` _hitactor))
      (`KismetSystemLibrary.DrawDebugSphere` _impactpoint 10.0 24 (struct :`R` 0.097318 :`G` 1.0 :`A` 1.0) 3.0 0.1)
      (bind _returnvalue_3 (`SculptedObject.VerticiesInRange` _assculpted_object _impactpoint 10.0))
      (`KismetSystemLibrary.PrintString` (`KismetStringLibrary.Conv_IntToString` _returnvalue_3)))))

(fn `UserConstructionScript`)